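; BP_Arme is a weapon that fires BP_Projectile actors automatically while firing is active.
; StartFiring passes a DoOnce gate, fires at once, then starts a looping timer at a rate set by ProjectileParSecondes.
; Each shot spawns a projectile at the PointSpawnProjectile transform and plays a 2D pistol sound.
; StopFiring clears the timer and resets the gate, so restarting fires immediately with no rate limit between presses.
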(event `FireProjectile`
  ;[1 1 1] Apparition projectile
  (`|SpawnActorFromClass` "/Game/Arme/BP_Projectile.BP_Projectile_C" (`SceneComponent.K2_GetComponentToWorld` (`self.PointSpawnProjectile`)) "Undefined" "OverrideRootScale" null null)
  (`GameplayStatics.PlaySound2D` "/Game/MilitaryWeapSilver/Sound/Pistol/Wavs/PistolA_Fire05.PistolA_Fire05" 1.0 1.0 0.0 null null))

(event `StartFiring`
  ;[1 1 1] Fréquence de tir de projectile
  (`/Engine/EditorBlueprintResources/StandardMacros.DoOnce` false :!label _label
    (:`Completed`
      (`self.FireProjectile`)
      (`KismetSystemLibrary.K2_SetTimer` null "FireProjectile" (/ 1.0 (`self.Projectile Par Secondes`)) true))))

(event `Stop Firing`
  ;[1 1 1] Interrompre tir de projectile
  (`KismetSystemLibrary.K2_ClearTimer` null "FireProjectile")
  (goto _label :!via `Reset`))

(fn `UserConstructionScript`)